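; BP_Spawn_CosmicProjectile is a spawner actor from a stylized VFX pack that repeatedly launches BP_Cosmic_Projectile actors.
; On BeginPlay it waits a delay scaled by its Level, then spawns a projectile at its own location and rotation.
; It passes its Gravity, ImpulsePower and Level values to each projectile, then loops through a self-calling Again event to respawn on a fixed interval.
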(event `Again`
  (bind (_returnvalue_location _returnvalue_rotation) (`KismetMathLibrary.BreakTransform` (`self.GetTransform`)))
  (`KismetSystemLibrary.Delay` 9.0)
  (`|SpawnActorFromClass` "/Game/ExternalContent/Stylized_VFX_StPack/Blueprints/UPDATE_1_2/BP_Cosmic_Projectile.BP_Cosmic_Projectile_C" (`KismetMathLibrary.MakeTransform` _returnvalue_location _returnvalue_rotation) "Undefined" "OverrideRootScale" null (`self.Gravity`) (`self.Impulse Power`) (`self.Level`) null :!label _label)
  (`self.Again`))

(event `self.ReceiveBeginPlay`
  (`KismetSystemLibrary.Delay` (* (`self.Level`) 3.0))
  (goto _label))

(fn `UserConstructionScript`)