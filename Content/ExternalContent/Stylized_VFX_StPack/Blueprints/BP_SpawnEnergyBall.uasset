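; Spawner actor from a stylized VFX pack that repeatedly launches BP_EnergyBall actors from its own location and rotation.
; BeginPlay waits for a delay scaled by Level, so spawners with different levels start staggered.
; Each spawn passes Gravity, ImpulsePower and Level to the ball, then calls the Again event, which loops endlessly on a fixed delay.
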(event `Again`
  (`KismetSystemLibrary.Delay` 4.5)
  (`|SpawnActorFromClass` "/Game/ExternalContent/Stylized_VFX_StPack/Blueprints/BP_EnergyBall.BP_EnergyBall_C" (`KismetMathLibrary.MakeTransform` (`self.K2_GetActorLocation`) (`self.K2_GetActorRotation`)) "Undefined" "OverrideRootScale" null 1.0 (`self.Gravity`) (`self.ImpulsePower`) (`self.Level`) true null :!label _label)
  (`self.Again`))

(event `self.ReceiveBeginPlay`
  (`KismetSystemLibrary.Delay` (* (`self.Level`) 1.5))
  (goto _label))

(fn `UserConstructionScript`)