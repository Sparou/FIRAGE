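; BP_VR_PickUp_02 is an animated pickup visual from a stylized VFX pack, tinted by a single Color variable.
; BeginPlay applies Color to the point light, a dynamic mesh material and, multiplied by Boost, the PickUpEffect particles.
; Timelines then drive material Power, vertical movement and scale relative to the starting transform, while Tick spins the mesh at a frame-rate-dependent rate.
; The light-intensity timeline is never triggered.
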(event `self.ReceiveBeginPlay`
  (`LightComponent.SetLightColor` (`self.PointLight`) (`self.Color`) true)
  (bind _returnvalue (`PrimitiveComponent.CreateDynamicMaterialInstance` (`self.StaticMesh`) 0 "/Game/ExternalContent/Stylized_VFX_StPack/VR/VR_Materials/M_VR_PickUp.M_VR_PickUp" "None"))
  (bind _output_get (set `self.Material` _returnvalue))
  (`MaterialInstanceDynamic.SetVectorParameterValue` _output_get "Color" (`self.Color`))
  (`FXSystemComponent.SetColorParameter` (`self.PickUpEffect`) "User.Color" (* (`self.Color`) (`self.Boost`)))
  (set `self.Location` (`SceneComponent.K2_GetComponentLocation` (`self.StaticMesh`)))
  (`|ExecutionSequence`
    (:`then_0`
      (bind (_direction _power _movement) (`Timeline|Power` :!via `PlayFromStart`)
        (:`Update`
          (`MaterialInstanceDynamic.SetScalarParameterValue` (`self.Material`) "Power" _power)
          (`SceneComponent.K2_SetWorldLocation` (`self.StaticMesh`) (`KismetMathLibrary.MakeVector` (.x (`self.Location`)) (.y (`self.Location`)) (+ _movement (.z (`self.Location`)))) false true))))
    (:`then_1`
      (set `self.StartScale` (`SceneComponent.K2_GetComponentScale` (`self.StaticMesh`)))
      (bind (_direction_2 _scale) (`Timeline|Scale` :!via `PlayFromStart`)
        (:`Update`
          (`SceneComponent.SetWorldScale3D` (`self.StaticMesh`) (* (`self.StartScale`) _scale)))))))

(event `self.ReceiveTick`
  (params (DeltaSeconds :type "Float (single-precision)"))
  (`SceneComponent.K2_AddLocalRotation` (`self.StaticMesh`) (struct :`Yaw` -0.5) false false))

(fn `UserConstructionScript`)